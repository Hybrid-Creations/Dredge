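; Player controller for Dredge that handles character selection, respawning, ready checks and UI display.
; On local BeginPlay it loads the chosen character from the game instance; spawn events respawn through the game mode, saving any new choice back to the instance.
; Ready state is passed to the TravelManager for an all-ready check.
; Escape toggles the menu, and Slash kills the controlled pawn through its health component.
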(event `self.ReceiveBeginPlay`
  (bind _asdredge_game_instance (cast `/Game/Blueprints/Defaults/DredgeGameInstance` (`GameplayStatics.GetGameInstance`) :!pure true))
  (`WidgetBlueprintLibrary.SetInputMode_GameOnly` self)
  (set `self.bShowMouseCursor` true)
  (if (`self.IsLocalPlayerController`)
    (set `self.MyCharacter` (`/Game/Blueprints/Defaults/DredgeGameInstance.MyCharacter` _asdredge_game_instance))
    (set `self.MyChosenCharacter` (`/Game/Blueprints/Defaults/DredgeGameInstance.MyChosenCharacter` _asdredge_game_instance))
    (`/Game/Blueprints/Defaults/DredgeGameInstance.Show AllGameSettings` (cast `/Game/Blueprints/Defaults/DredgeGameInstance` (`GameplayStatics.GetGameInstance`) :!pure true) true)))

(event `Key|Slash`
  (params (Key :type "Key Structure" :default "AnyKey"))
  (:`Pressed`
    (`/Game/Blueprints/Defaults/Gameplay/Health/HealthComponent.Death` (`self.GetComponentByClass` (`self.K2_GetPawn`) "/Game/Blueprints/Defaults/Gameplay/Health/PlayerHealthComponent.PlayerHealthComponent_C") (0.0 0.0 5.0))))

(event `Key|Escape`
  (params (Key :type "Key Structure" :default "AnyKey"))
  (:`Pressed`
    (bind _asdredge_game_instance (cast `/Game/Blueprints/Defaults/DredgeGameInstance` (`GameplayStatics.GetGameInstance`)))
    (`/Game/Blueprints/Defaults/DredgeGameInstance.Toggle Esc Menu` _asdredge_game_instance)))

(event `ShowReadyUI`
  (bind _returnvalue (`|CreateWidget` "/Game/WorldManipulation/Travel/UI/ReadyCheck.ReadyCheck_C" self))
  (`UserWidget.AddToViewport` _returnvalue 50))

(event `SetReady`
  (params (ReadyToTravel :type Boolean))
  (set `self.ReadyToTravel` ReadyToTravel)
  (bind _outactors (`GameplayStatics.GetAllActorsOfClass` "/Game/WorldManipulation/Travel/TravelManager.TravelManager_C"))
  (`/Game/WorldManipulation/Travel/TravelManager.CheckIfAllReady` (`|GetArrayItem` _outactors)))

(event `ShowLoadingScreen`
  (`/Game/Tools/Global/GlobalFunctionLib.CreateLoadingScreen` self))

(event `Spawn With New Character Server`
  (params (MyCharacter :type "/Game/Characters/DredgeCharacter Class Reference") (MyChosenCharacter :type "/Game/Characters/CharacterManipulation/SelectedCharacter Enum"))
  (bind _asdredge_game_mode (cast `/Game/Blueprints/Defaults/DredgeGameMode` (`GameplayStatics.GetGameMode`)))
  (set `self.MyCharacter` MyCharacter)
  (set `self.MyChosenCharacter` MyChosenCharacter)
  (`self.Set My Character` MyCharacter MyChosenCharacter)
  (`/Game/Blueprints/Defaults/DredgeGameMode.Respawn` _asdredge_game_mode self))

(event `SpawnCharacterServer`
  (`/Game/Blueprints/Defaults/DredgeGameMode.Respawn` (cast `/Game/Blueprints/Defaults/DredgeGameMode` (`GameplayStatics.GetGameMode`) :!pure true) self))

(event `Set My Character`
  (params (MyCharacter :type "/Game/Characters/DredgeCharacter Class Reference") (MyChosenCharacter :type "/Game/Characters/CharacterManipulation/SelectedCharacter Enum"))
  (bind _asdredge_game_instance (cast `/Game/Blueprints/Defaults/DredgeGameInstance` (`GameplayStatics.GetGameInstance`) :!pure true))
  (set `/Game/Blueprints/Defaults/DredgeGameInstance.MyCharacter` MyCharacter _asdredge_game_instance)
  (set `/Game/Blueprints/Defaults/DredgeGameInstance.MyChosenCharacter` MyChosenCharacter _asdredge_game_instance))

(event `Show MainUI`
  (bind _asdredge_main_hud (cast `/Game/UI/Game/DredgeMainHUD` (`self.GetHUD`)))
  (`/Game/UI/Game/DredgeMainHUD.Show Main UI` _asdredge_main_hud))

(fn `OnRep_MyChosenCharacter`)

(fn `UserConstructionScript`)