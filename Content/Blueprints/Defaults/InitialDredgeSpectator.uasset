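; InitialDredgeSpectator is the player's starting spectator, handling the hand-off from loading screen to playable character.
; After a short BeginPlay delay it prepares and continues the waiting loading screen with SpawnCharacter as callback, or calls SpawnCharacter directly if none exists.
; If the controller's MyCharacter is base DredgeCharacter, it finds or spawns a ChangeCharacterManager and focuses the character selection UI.
; Otherwise it calls SpawnCharacterServer on the DredgePlayerController.
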(event `self.ReceiveBeginPlay`
  (`KismetSystemLibrary.Delay` 0.2)
  (bind _loadingscreen (`/Game/Tools/Global/GlobalFunctionLib.PrepareLoadingScreenForContinue` self (delegate `Spawn Character`)))
  (bind _output_get (set `self.LoadingScreenWaiting` _loadingscreen))
  (`/Engine/EditorBlueprintResources/StandardMacros.IsValid` _output_get
    (:`Is Valid`
      (`/Game/Tools/Global/GlobalFunctionLib.ContinueLoadingScreen` (`self.LoadingScreenWaiting`)))
    (:`Is Not Valid`
      (`self.Spawn Character`))))

(event `Key|AnyKey`
  (params (Key :type "Key Structure")))

(event `Spawn Character`
  (bind _returnvalue (`self.GetController`))
  (bind _asdredge_player_controller (cast `/Game/Blueprints/Defaults/DredgePlayerController` (`self.GetController`) :!pure true))
  (bind _mycharacter (`/Game/Blueprints/Defaults/DredgePlayerController.MyCharacter` _asdredge_player_controller))
  (`|ExecutionSequence`
    (:`then_0`
      (`KismetSystemLibrary.PrintString` (`KismetSystemLibrary.GetClassDisplayName` _mycharacter) true true (struct :`G` 0.66 :`B` 1.0 :`A` 1.0) 5.0)
      (if (== _mycharacter "/Game/Characters/DredgeCharacter.DredgeCharacter_C")
        (bind _outactors (`GameplayStatics.GetAllActorsOfClass` "/Game/Characters/CharacterManipulation/ChangeCharacterManager.ChangeCharacterManager_C"))
        (bind _output (`|GetArrayItem` _outactors))
        (`/Engine/EditorBlueprintResources/StandardMacros.IsValid` _output
          (:`Is Valid`
            (`/Game/Characters/CharacterManipulation/ChangeCharacterManager.ShowChangeCharacterUI` _output _returnvalue))
          (:`Is Not Valid`
            (bind _returnvalue_2 (`|SpawnActorFromClass` "/Game/Characters/CharacterManipulation/ChangeCharacterManager.ChangeCharacterManager_C" (`KismetMathLibrary.MakeTransform` (0.0 0.0 -1000.0)) "Undefined" "OverrideRootScale" null null))
            (`/Game/Characters/CharacterManipulation/ChangeCharacterManager.ShowChangeCharacterUI` _returnvalue_2 _returnvalue)))
        (`KismetSystemLibrary.Delay` 0.1)
        (bind _foundwidgets (`WidgetBlueprintLibrary.GetAllWidgetsOfClass` "/Game/Characters/CharacterManipulation/ChooseCharacterUI.ChooseCharacterUI_C"))
        (`WidgetBlueprintLibrary.SetInputMode_GameAndUIEx` (cast `PlayerController` (`self.GetController`) :!pure true) (`|GetArrayItem` _foundwidgets) "DoNotLock" false)
        (else
          (`/Game/Blueprints/Defaults/DredgePlayerController.SpawnCharacterServer` _asdredge_player_controller))))))

(fn `UserConstructionScript`)