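; DredgeGameInstance is the game instance that manages front-end menus and multiplayer session hosting.
; Show events lazily create and cache the server browser, main menu, host menu and loading screen widgets.
; StartNewSession creates an Advanced Session carrying server name, password and host name as extra settings, then opens Lobby as a listen server.
; StartGame shows the loading screen and server-travels to the Town map.
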(event `Show Server Browser`
  ;[1 1 1] Show Server Browser
  (`/Engine/EditorBlueprintResources/StandardMacros.IsValid` (`self.ServerBrowserWdgt`)
    (:`Is Valid`
      _)
    (:`Is Not Valid`
      (bind _returnvalue (`|CreateWidget` "/Game/Art/UI/ServerBrowser.ServerBrowser_C"))
      (bind _output_get (set `self.ServerBrowserWdgt` _returnvalue))))
  (`UserWidget.AddToViewport` _output_get 1))

(event `Show MainMenu`
  ;[1 1 1] Show Main Menu
  (`/Engine/EditorBlueprintResources/StandardMacros.IsValid` (`self.MainMenuWdgt`)
    (:`Is Valid`
      _)
    (:`Is Not Valid`
      (bind _returnvalue (`|CreateWidget` "/Game/Art/UI/MainGameMenu.MainGameMenu_C"))
      (bind _output_get (set `self.MainMenuWdgt` _returnvalue))))
  (`UserWidget.AddToViewport` _output_get 1)
  (`Widget.SetVisibility` (`/Game/Art/UI/MainGameMenu.ServerSetupWindow` _output_get) "Hidden"))

(event `Show HostMenu`
  ;[1 1 1] Show The Hosting Menu (After creatiion of session)
  (`/Engine/EditorBlueprintResources/StandardMacros.IsValid` (`self.HostMenuWdgt`)
    (:`Is Valid`
      _)
    (:`Is Not Valid`
      (bind _returnvalue (`|CreateWidget` "/Game/Art/UI/HostMenu.HostMenu_C"))
      (bind _output_get (set `self.HostMenuWdgt` _returnvalue))))
  (`UserWidget.AddToViewport` _output_get 1))

(event `ShowLoadingScreen`
  ;[1 1 1] Show the Loading Screen
  (`/Engine/EditorBlueprintResources/StandardMacros.IsValid` (`self.CurrentLoadingScreen`)
    (:`Is Valid`
      _)
    (:`Is Not Valid`
      (bind _returnvalue (`|CreateWidget` "/Game/Art/UI/LoadingScreen.LoadingScreen_C"))
      (bind _output_get (set `self.CurrentLoadingScreen` _returnvalue))))
  (`UserWidget.AddToViewport` _output_get 99))

(event `Start New Session`
  (params (ServerName :type String) (Password :type String) (HostName :type String))
  ;[1 1 1] Start New Game
  (`self.ShowLoadingScreen`)
  (`CreateSessionCallbackProxyAdvanced.CreateAdvancedSession` (`|MakeArray` (`AdvancedSessionsLibrary.MakeLiteralSessionPropertyString` "SERVERNAME" ServerName) (`AdvancedSessionsLibrary.MakeLiteralSessionPropertyString` "PASSWORD" Password) (`AdvancedSessionsLibrary.MakeLiteralSessionPropertyString` "HOSTNAME" HostName)) (`GameplayStatics.GetPlayerController` 0) 4
    (:`OnSuccess`
      (`WidgetLayoutLibrary.RemoveAllWidgets`)
      (`GameplayStatics.OpenLevel` "Lobby" true "listen"))
    (:`OnFailure`
      (`KismetSystemLibrary.PrintString` "Fail Create Session" true true (struct :`R` 1.0 :`A` 1.0)))))

(event `Start Game`
  (`self.ShowLoadingScreen`)
  (`KismetSystemLibrary.ExecuteConsoleCommand` (`KismetTextLibrary.Conv_TextToString` (`|FormatText` "servertravel /Game/Maps/Town"))))