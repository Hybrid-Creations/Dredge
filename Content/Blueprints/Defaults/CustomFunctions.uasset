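; Custom function asset providing a Sort function that orders an array using each element's CompareTo.
; It runs an iterative bottom-up merge sort, doubling the block size each pass via an incremental for-loop.
; Adjacent blocks merge into a holding array, which is copied back into the target after each pass.
; The array length is printed before and after sorting, and the target array is returned.
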(fn `Sort`
  (params (TargetArray :type "Array of /Game/Blueprints/Defaults/Comparable Interface"))
  (returns (SortedArray :type "Array of /Game/Blueprints/Defaults/Comparable Interface"))
  (locals (BlockSize :type Integer :default 1) (HoldingArray :type "Array of /Game/Blueprints/Defaults/Comparable Interface") (FirstPosition :type Integer) (SecondPosition :type Integer) (Left :type Integer) (Right :type Integer) (End :type Integer) (i :type Integer) (j :type Integer))
  (bind _returnvalue (`KismetArrayLibrary.Array_Length` TargetArray))
  (bind _targetarray (`local.TargetArray`))
  (bind _targetarray_2 (`local.TargetArray`))
  (`KismetSystemLibrary.PrintString` null (`KismetStringLibrary.Conv_IntToString` _returnvalue))
  (`KismetArrayLibrary.Array_Resize` (`local.HoldingArray`) _returnvalue)
  (while (< (`local.BlockSize`) _returnvalue)
    (bind _index (`/Game/Blueprints/Defaults/CustomMacros.IncrementalForLoop` 0 (- _returnvalue 1) (* 2 (`local.BlockSize`)))
      (:`Loop Body`
        (bind _output_get (set `local.Left` _index))
        (set `local.i` _output_get)
        (bind _output_get_2 (set `local.Right` (`KismetMathLibrary.Min` _returnvalue (+ _index (`local.BlockSize`)))))
        (set `local.j` _output_get_2)
        (set `local.End` (`KismetMathLibrary.Min` _returnvalue (+ _index (* 2 (`local.BlockSize`)))))
        (for _index_2 (range (`local.Left`) (`local.End`))
          (bind _result (`/Game/Blueprints/Defaults/Comparable.CompareTo` (`|GetArrayItem` _targetarray (`local.i`)) (`|GetArrayItem` _targetarray (`local.j`))))
          (if (and (or (<= _result 0) (>= (`local.j`) (`local.End`))) (< (`local.i`) (`local.Right`)))
            (`KismetArrayLibrary.Array_Set` (`local.HoldingArray`) _index_2 (`|GetArrayItem` (`local.TargetArray`) (`local.i`)))
            (set `local.i` (+ 1 (`local.i`)))
            (else
              (`KismetArrayLibrary.Array_Set` (`local.HoldingArray`) _index_2 (`|GetArrayItem` (`local.TargetArray`) (`local.j`)))
              (set `local.j` (+ 1 (`local.j`)))))))
      (:`Completed`
        (set `local.BlockSize` (* 2 (`local.BlockSize`)))
        (for (_array_element _array_index) (`local.HoldingArray`)
          (`KismetArrayLibrary.Array_Set` (`local.TargetArray`) _array_index _array_element)))))
  (`KismetSystemLibrary.PrintString` null (`KismetStringLibrary.Conv_IntToString` (`KismetArrayLibrary.Array_Length` _targetarray_2)))
  (return _targetarray_2))