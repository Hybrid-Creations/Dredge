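; Game mode for Dredge that tracks player controllers and handles their respawning and shared loading screen.
; Player spawn points are gathered at BeginPlay, with a lookup that supplies a random one for each respawn.
; Respawn destroys the current pawn, then spawns and possesses the controller's character class at that location.
; It then rebuilds every player's chosen character list and pushes it to the level's ChangeCharacterManager.
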(event `self.K2_PostLogin`
  (params (NewPlayer :type "PlayerController Object Reference"))
  (`KismetArrayLibrary.Array_AddUnique` (`self.AllPlayers`) NewPlayer))

(event `self.K2_OnSwapPlayerControllers`
  (params (OldPC :type "PlayerController Object Reference") (NewPC :type "PlayerController Object Reference"))
  (`KismetArrayLibrary.Array_AddUnique` (`self.AllPlayers`) NewPC))

(event `self.ReceiveBeginPlay`
  (`self.Get All Spawn Points`))

(event `Respawn`
  (params (Controller :type "PlayerController Object Reference"))
  (bind _returnvalue (`Controller.K2_GetPawn` Controller))
  (bind (_allspawnpoints _onerandompoint) (`self.Check If Spawn Points Are Cached`))
  (`/Engine/EditorBlueprintResources/StandardMacros.IsValid` _returnvalue
    (:`Is Valid`
      (`self.K2_DestroyActor` _returnvalue))
    (:`Is Not Valid`
      _))
  (bind _returnvalue_2 (`|SpawnActorFromClass` (`/Game/Blueprints/Defaults/DredgePlayerController.MyCharacter` (cast `/Game/Blueprints/Defaults/DredgePlayerController` Controller :!pure true)) (`KismetMathLibrary.Conv_VectorToTransform` (`self.K2_GetActorLocation` _onerandompoint)) "AdjustIfPossibleButAlwaysSpawn" "OverrideRootScale" Controller))
  (`Controller.Possess` Controller _returnvalue_2)
  (`KismetArrayLibrary.Array_Clear` (`self.ChosenCharacters`))
  (for _array_element (`self.AllPlayers`)
    (bind _asdredge_player_controller (cast `/Game/Blueprints/Defaults/DredgePlayerController` _array_element))
    (`KismetArrayLibrary.Array_Add` (`self.ChosenCharacters`) (`/Game/Blueprints/Defaults/DredgePlayerController.MyChosenCharacter` _asdredge_player_controller)))
  (bind _outactors (`GameplayStatics.GetAllActorsOfClass` "/Game/Characters/CharacterManipulation/ChangeCharacterManager.ChangeCharacterManager_C"))
  (set `/Game/Characters/CharacterManipulation/ChangeCharacterManager.ChosenCharacters` (`self.ChosenCharacters`) (`|GetArrayItem` _outactors)))

(event `ShowLoadingScreenAll`
  (for _array_element (`self.AllPlayers`)
    (bind _asdredge_player_controller (cast `/Game/Blueprints/Defaults/DredgePlayerController` _array_element))
    (`/Game/Blueprints/Defaults/DredgePlayerController.ShowLoadingScreen` _asdredge_player_controller)))

(fn `UserConstructionScript`)