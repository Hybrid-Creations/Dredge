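; AudioManager Blueprint that controls background music playback through a single BGM audio component.
; SwapBGM fades the current track out, waits for the fade duration, sets the new sound and fades it back in to the stored BGMVolume.
; Functions also start playback with an optional new track and update the volume multiplier.
; The playback-percent event is an empty testing hook, with its debug print left disconnected.
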(event `Swap BGM`
  (params (`New BGM` :type "SoundBase Object Reference") (FadeDuration :type "Float (double-precision)"))
  (`self.Fade Out BGM` FadeDuration)
  (`KismetSystemLibrary.Delay` FadeDuration)
  (`AudioComponent.SetSound` (`self.BGM`) `New BGM`)
  (`self.Fade In BGM` FadeDuration))

(event `self.BGM.OnAudioPlaybackPercent`
  (params (PlayingSoundWave :type "SoundWave Object Reference") (PlaybackPercent :type "Float (single-precision)"))
  ;[1 1 1] For Testing If Playing
)

(event `Fade Out BGM`
  (params (FadeDuration :type "Float (double-precision)"))
  (`AudioComponent.FadeOut` (`self.BGM`) FadeDuration 0.0))

(event `Fade In BGM`
  (params (`Fade Duration` :type "Float (double-precision)"))
  (`AudioComponent.FadeIn` (`self.BGM`) `Fade Duration` (`self.BGMVolume`) 0.0))

(fn `Play BGM`
  (params (NewBGM :type "SoundBase Object Reference"))
  (bind _bgm (`self.BGM`))
  (`/Engine/EditorBlueprintResources/StandardMacros.IsValid` NewBGM
    (:`Is Valid`
      (`AudioComponent.SetSound` _bgm NewBGM))
    (:`Is Not Valid`
      _))
  (`AudioComponent.Play` _bgm 0.0))

(fn `Set BGM Volume`
  (params (BGMVolume :type "Float (double-precision)"))
  (bind _output_get (set `self.BGMVolume` BGMVolume))
  (`AudioComponent.SetVolumeMultiplier` (`self.BGM`) _output_get))

(fn `UserConstructionScript`)