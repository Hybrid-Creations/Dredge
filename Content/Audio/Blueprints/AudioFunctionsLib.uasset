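; Blueprint function library of background music helpers that forward swap and fade requests to the game instance.
; Each function casts the supplied game instance to DredgeGameInstance, which does the actual BGM work.
; SwapBGM plays either a new track or the instance's saved CurrentBGM, depending on a flag, with a fade duration.
; The fade-in and fade-out helpers pass their duration through and return it.
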(fn `Fade In BGM`
  (params (`Game Instance` :type "GameInstance Object Reference") (Duration :type "Float (double-precision)"))
  (returns (`Duration ` :type "Float (double-precision)"))
  (bind _asdredge_game_instance (cast `/Game/Blueprints/Defaults/DredgeGameInstance` `Game Instance`))
  (`/Game/Blueprints/Defaults/DredgeGameInstance.Fade In BGM` _asdredge_game_instance Duration)
  (return Duration))

(fn `Fade Out BGM`
  (params (GameInstance :type "GameInstance Object Reference") (Duration :type "Float (double-precision)"))
  (returns (`Duration ` :type "Float (double-precision)"))
  (bind _asdredge_game_instance (cast `/Game/Blueprints/Defaults/DredgeGameInstance` GameInstance))
  (`/Game/Blueprints/Defaults/DredgeGameInstance.Fade Out BGM` _asdredge_game_instance Duration)
  (return Duration))

(fn `Swap BGM`
  (params (GameInstance :type "GameInstance Object Reference") (`New BGM` :type "SoundBase Object Reference") (`Use Saved BGM` :type Boolean) (FadeDuration :type "Float (double-precision)"))
  (bind _asdredge_game_instance (cast `/Game/Blueprints/Defaults/DredgeGameInstance` GameInstance))
  (if `Use Saved BGM`
    (`/Game/Blueprints/Defaults/DredgeGameInstance.Swap BGM` _asdredge_game_instance (`/Game/Blueprints/Defaults/DredgeGameInstance.CurrentBGM` _asdredge_game_instance) FadeDuration)
    (return)
    (else
      (`/Game/Blueprints/Defaults/DredgeGameInstance.Swap BGM` _asdredge_game_instance `New BGM` FadeDuration)
      (return))))